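; BP_bolt is a currency pickup actor that rewards the player with a random amount of Currency.
; When its Sphere overlaps a ThirdPersonCharacter, it waits briefly, then adds the random amount to the first player pawn's Currency and destroys itself.
; The reward always goes to player pawn 0, not necessarily the overlapping character.
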(event `self.Sphere.OnComponentBeginOverlap`
  (params (OverlappedComponent :type "PrimitiveComponent Object Reference") (OtherActor :type "Actor Object Reference") (OtherComp :type "PrimitiveComponent Object Reference") (OtherBodyIndex :type Integer) (bFromSweep :type Boolean) (SweepResult :type "HitResult Structure (by ref)"))
  (bind _asthird_person_character (cast `/Game/ThirdPersonBP/Blueprints/ThirdPersonCharacter` (`GameplayStatics.GetPlayerPawn` 0) :!pure true))
  (cast `/Game/ThirdPersonBP/Blueprints/ThirdPersonCharacter` OtherActor)
  (`KismetSystemLibrary.Delay` 1.0)
  (set `/Game/ThirdPersonBP/Blueprints/ThirdPersonCharacter.currency` (+ (`/Game/ThirdPersonBP/Blueprints/ThirdPersonCharacter.currency` _asthird_person_character) (`KismetMathLibrary.RandomIntegerInRange` 40 90)) _asthird_person_character)
  (`/Engine/EditorBlueprintResources/StandardMacros.IsValid` self
    (:`Is Valid`
      (`self.K2_DestroyActor`))))

(fn `UserConstructionScript`)