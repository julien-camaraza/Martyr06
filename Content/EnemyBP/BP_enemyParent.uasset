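; Base enemy Blueprint, going by its name, that takes damage through a hit event gated by an invincibility flag.
; EventHit ignores hits while Invincibility is set; otherwise it sets the flag, stores DamageTaken and subtracts it from Health.
; A separate InvincibiltyOver event clears the flag, with no timer or death check in this graph.
; BeginPlay only casts the player to ThirdPersonCharacter, and the SwordCollision lookup is unconnected.
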(event `self.ReceiveBeginPlay`
  (cast `/Game/ThirdPersonBP/Blueprints/ThirdPersonCharacter` (`GameplayStatics.GetPlayerCharacter` 0)))

(event `self.ReceiveActorBeginOverlap`
  (params (OtherActor :type "Actor Object Reference")))

(event `EventHit`
  (params (damageTaken :type "Float (double-precision)"))
  (if (not (`self.Invincibility`))
    (set `self.Invincibility` true)
    (set `self.damageTaken` damageTaken)
    (set `self.Health` (- (`self.Health`) (`self.damageTaken`)))))

(event `InvincibiltyOver`
  (set `self.Invincibility` false))

(fn `UserConstructionScript`)