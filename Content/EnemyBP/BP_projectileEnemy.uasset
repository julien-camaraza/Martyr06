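; BP_projectileEnemy is an enemy that, when its Shooting flag is set, fires a BP_projectileParent from its own transform every second with a laser sound.
; Its EventHit handler subtracts incoming damage from Health and grants a brief timer-based invincibility window after each non-lethal hit.
; At zero health it activates a Niagara hit effect, hides the mesh, disables mesh collision, then after a delay spawns a BP_bolt and destroys itself.
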(event `self.ReceiveBeginPlay`
  (`|ExecutionSequence`
    (:`then_0`
      (bind _asthird_person_character (cast `/Game/ThirdPersonBP/Blueprints/ThirdPersonCharacter` (`GameplayStatics.GetPlayerCharacter` 0)))
      (set `self.As Third Person Character` _asthird_person_character))
    (:`then_1`
      (if (`self.shooting`)
        (`KismetSystemLibrary.K2_SetTimerDelegate` (delegate `shootProjectile`) 1.0 true)))))

(event `shootProjectile`
  (bind _defaultsceneroot (`self.DefaultSceneRoot`))
  (`|SpawnActorFromClass` "/Game/EnemyBP/BP_projectileParent.BP_projectileParent_C" (`self.GetTransform`) "Undefined" "OverrideRootScale" null null)
  (`/Game/NewMacros.IsValid` _defaultsceneroot
    (:`Is Valid`
      (`GameplayStatics.PlaySoundAtLocation` "/Game/Sound/SoundEffects/RobotSounds/Weapons/cue_Laser.cue_Laser" (`SceneComponent.K2_GetComponentLocation` _defaultsceneroot) (struct) 1.0 1.0 0.0 null null null))))

(event `EventHit`
  (params (damageTaken :type "Float (double-precision)"))
  (if (not (`self.Invincibility`))
    (set `self.damageTaken` damageTaken)
    (set `self.Health` (- (`self.Health`) (`self.damageTaken`)))
    (if (<= (`self.Health`) 0.0)
      (`self.die`)
      (else
        (set `self.Invincibility` true)
        (`KismetSystemLibrary.K2_SetTimerDelegate` (delegate `vincible`) 0.5)))))

(event `vincible`
  (set `self.Invincibility` false))

(event `die`
  (bind _enemymesh (`self.enemyMesh`))
  (`ActorComponent.Activate` (`self.NS_ky_hit_fire`) false)
  (`SceneComponent.SetVisibility` _enemymesh false false)
  (`PrimitiveComponent.SetCollisionEnabled` _enemymesh "NoCollision")
  (`KismetSystemLibrary.Delay` 1.0)
  (`|SpawnActorFromClass` "/Game/CoreSystems/BP_bolt.BP_bolt_C" (`SceneComponent.K2_GetComponentToWorld` (`self.DefaultSceneRoot`)) "Undefined" "OverrideRootScale" null null)
  (`/Engine/EditorBlueprintResources/StandardMacros.IsValid` self
    (:`Is Valid`
      (`self.K2_DestroyActor`))))

(fn `UserConstructionScript`)