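; Base enemy projectile Blueprint that can be blocked and parried by the third-person character.
; Blocked runs a timeline window that sends a parry message once if the player stops blocking, then calls Die.
; GetParried clears the Evil flag, plays feedback, flags the player as parrying and redirects velocity along a fixed world axis.
; A despawn timer also calls Die, which only destroys projectiles still marked Evil.
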(event `Blocked`
  (params (ThirdPersonCharacter :type "/Game/ThirdPersonBP/Blueprints/ThirdPersonCharacter Object Reference"))
  (set `self.isBlocked` true)
  (`Timeline|checkForParry` :!via `PlayFromStart`
    (:`Update`
      (if (not (`/Game/ThirdPersonBP/Blueprints/ThirdPersonCharacter.isBlocking` ThirdPersonCharacter))
        (`/Engine/EditorBlueprintResources/StandardMacros.DoOnce` false
          (:`Completed`
            (message `/Game/Animations/MainCharacter/EnemyInterface.GetParried` self)))))
    (:`Finished`
      (`self.Die`))))

(event `/Game/Animations/MainCharacter/EnemyInterface.GetParried`
  (set `self.Evil` false)
  (`KismetSystemLibrary.PrintString` "Parried")
  (`GameplayStatics.PlaySound2D` "/Game/Sound/SoundEffects/RobotSounds/Weapons/CUE_parry.CUE_parry" 1.0 1.0 0.0 null null)
  (set `/Game/ThirdPersonBP/Blueprints/ThirdPersonCharacter.isParrying` true (stale `Blocked` ThirdPersonCharacter))
  (set `MovementComponent.Velocity` (0.0 -1000.0 0.0) (`self.ProjectileMovement`)))

(event `self.ReceiveBeginPlay`
  (`KismetSystemLibrary.K2_SetTimerDelegate` (delegate `Die`) (`self.DespawnTime`)))

(event `Die`
  (if (`self.Evil`)
    (`/Engine/EditorBlueprintResources/StandardMacros.IsValid` self
      (:`Is Valid`
        (`self.K2_DestroyActor`)))))

(fn `UserConstructionScript`)