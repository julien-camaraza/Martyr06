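; Final boss Blueprint with two swinging arms that damage BP_Martyr on overlap and a weak point that takes hits.
; Timeline-driven pivot rotations form hook, crush and two-arm smash attacks, gated by hand-in-use flags, with camera shake and crack decals.
; A looping timer picks attacks, but its random range reaches only the hooks.
; As wired, BeginPlay immediately calls Die, as does any weak-point hit, enabling physics and spawning BP_finishLevel.
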(event `turnOn`
  (`KismetSystemLibrary.K2_SetTimerDelegate` (delegate `chooseAttack`) 2.0 true)
  (`self.chooseAttack`))

(event `chooseAttack`
  (switch `int` (`KismetMathLibrary.RandomIntegerInRange` 0 1)
    (:`0`
      (`self.leftHook`)
      (`KismetSystemLibrary.PrintString` "leftHook"))
    (:`1`
      (`self.rightHook`)
      (`KismetSystemLibrary.PrintString` "rightHook"))
    (:`2`
      (`self.leftCrush`)
      (`KismetSystemLibrary.PrintString` "leftCrush"))
    (:`3`
      (`self.rightCrush`)
      (`KismetSystemLibrary.PrintString` "rightCrush"))
    (:`4`
      (`self.tryToRapidSmash` :!label _label)
      (`KismetSystemLibrary.PrintString` "rapidSmahs"))
    (:`5`
      (goto _label))
    (:`6`
      (goto _label))
    (:`7`
      (goto _label))))

(event `Die`
  (`GameplayStatics.PlaySoundAtLocation` "/Game/Sound/boss/CUE_bossDie.CUE_bossDie" (`SceneComponent.K2_GetComponentLocation` (`self.DefaultSceneRoot`)) (struct) 1.0 1.0 0.0 null null null)
  (`ActorComponent.Activate` (`self.damage`) false)
  (`GameplayStatics.PlaySoundAtLocation` "/Game/Sound/boss/CUE_bossExplode.CUE_bossExplode" (`SceneComponent.K2_GetComponentLocation` (`self.DefaultSceneRoot`)) (struct) 1.0 1.0 0.0 null null null)
  (`KismetSystemLibrary.Delay` 0.05)
  (`ActorComponent.Activate` (`self.damage1`) false)
  (`GameplayStatics.PlaySoundAtLocation` "/Game/Sound/boss/CUE_bossExplode.CUE_bossExplode" (`SceneComponent.K2_GetComponentLocation` (`self.DefaultSceneRoot`)) (struct) 1.0 1.0 0.0 null null null)
  (`KismetSystemLibrary.Delay` 0.05)
  (`ActorComponent.Activate` (`self.damage2`) false)
  (`GameplayStatics.PlaySoundAtLocation` "/Game/Sound/boss/CUE_bossExplode.CUE_bossExplode" (`SceneComponent.K2_GetComponentLocation` (`self.DefaultSceneRoot`)) (struct) 1.0 1.0 0.0 null null null)
  (`KismetSystemLibrary.Delay` 0.05)
  (`ActorComponent.Activate` (`self.damage3`) false)
  (`GameplayStatics.PlaySoundAtLocation` "/Game/Sound/boss/CUE_bossExplode.CUE_bossExplode" (`SceneComponent.K2_GetComponentLocation` (`self.DefaultSceneRoot`)) (struct) 1.0 1.0 0.0 null null null)
  (`KismetSystemLibrary.Delay` 0.05)
  (`|SpawnActorFromClass` "/Game/SideScrollerBP/Blueprints/BP_finishLevel.BP_finishLevel_C" (`self.GetTransform`) "Undefined" "OverrideRootScale" null null)
  (`PrimitiveComponent.SetSimulatePhysics` (`self.Cube`) true)
  (`PrimitiveComponent.SetSimulatePhysics` (`self.LeftArm`) true)
  (`PrimitiveComponent.SetSimulatePhysics` (`self.RightArm`) true))

(event `self.ReceiveBeginPlay`
  (`self.Die`))

(event `takeDamage`
  (params (damageTaken :type "Float (double-precision)") (hitLocation :type "ActorComponent Object Reference"))
  (bind _cube (`self.Cube`))
  (if (== hitLocation (`self.weakPoint`))
    (set `self.health` (- (`self.health`) damageTaken))
    (if true
      (`self.Die`)
      (else
        (`GameplayStatics.PlaySoundAtLocation` "/Game/Sound/boss/CUE_bossPain.CUE_bossPain" (`SceneComponent.K2_GetComponentLocation` (`self.Cube`)) (struct) 1.0 1.0 0.0 null null null)
        (`/Engine/EditorBlueprintResources/StandardMacros.DoOnce` false
          (:`Completed`
            (bind (_direction _newtrack_0) (`Timeline|moveBackwards` :!via `PlayFromStart`)
              (:`Update`
                (bind (_returnvalue_location _returnvalue_rotation) (`KismetMathLibrary.BreakTransform` (`SplineComponent.GetTransformAtDistanceAlongSpline` (`self.followSpline`) (`KismetMathLibrary.Lerp` 0.0 (`SplineComponent.GetSplineLength` (`self.followSpline`)) _newtrack_0) "World" false)))
                (`SceneComponent.K2_SetWorldLocation` _cube _returnvalue_location false false)
                (`SceneComponent.K2_SetWorldRotation` _cube _returnvalue_rotation false false)))))))))

(event `leftHook`
  (if (not (`self.leftHandInUse`))
    (set `self.leftHandInUse` true)
    (bind (_direction _newtrack_0) (`Timeline|leftHookTimeline` :!via `PlayFromStart`)
      (:`Update`
        (`SceneComponent.K2_SetRelativeRotation` (`self.leftArmPivotPoint`) (`KismetMathLibrary.RLerp` (`self.leftArmStartingRotation`) (`self.leftArmHookRotation`) _newtrack_0) false false))
      (:`Finished`
        (set `self.leftHandInUse` false))
      (:`NewTrack_1`
        (`GameplayStatics.PlayWorldCameraShake` "/Game/CoreSystems/BP_camerashake.BP_camerashake_C" (0.0 0.0 0.0) 0.0 (`self.Outer Radius`))
        (`GameplayStatics.PlaySoundAtLocation` "/Game/Sound/boss/CUE_swingBoss.CUE_swingBoss" (`SceneComponent.K2_GetComponentLocation` (`self.leftHookCollision`)) (struct) 1.0 1.0 0.0 null null null))
      (:`collision`
        (`/Engine/EditorBlueprintResources/StandardMacros.FlipFlop`
          (:`A`
            (`PrimitiveComponent.SetCollisionEnabled` (`self.leftHookCollision`) "QueryOnly"))
          (:`B`
            (`PrimitiveComponent.SetCollisionEnabled` (`self.leftHookCollision`) "NoCollision")))))))

(event `rightHook`
  (bind _righthookcollision (`self.rightHookCollision`))
  (if (not (`self.rightHandInUse`))
    (set `self.rightHandInUse` true)
    (bind (_direction _newtrack_0) (`Timeline|rightHookTimeline` :!via `PlayFromStart`)
      (:`Update`
        (`SceneComponent.K2_SetRelativeRotation` (`self.rightArmPivotPoint`) (`KismetMathLibrary.RLerp` (`self.rightArmStartingRotation`) (`self.rightArmHookRotation`) _newtrack_0) false false))
      (:`Finished`
        (set `self.rightHandInUse` false))
      (:`NewTrack_1`
        (`GameplayStatics.PlayWorldCameraShake` "/Game/CoreSystems/BP_camerashake.BP_camerashake_C" (0.0 0.0 0.0) 0.0 (`self.Outer Radius`))
        (`GameplayStatics.PlaySoundAtLocation` "/Game/Sound/boss/CUE_swingBoss.CUE_swingBoss" (`SceneComponent.K2_GetComponentLocation` (`self.rightHookCollision`)) (struct) 1.0 1.0 0.0 null null null))
      (:`NewTrack_2`
        (`/Engine/EditorBlueprintResources/StandardMacros.FlipFlop`
          (:`A`
            (`PrimitiveComponent.SetCollisionEnabled` _righthookcollision "QueryOnly"))
          (:`B`
            (`PrimitiveComponent.SetCollisionEnabled` _righthookcollision "NoCollision")))))))

(event `leftCrush`
  (bind _rightcrushcollision (`self.rightCrushCollision`))
  (if (not (`self.leftHandInUse`))
    (set `self.leftHandInUse` true)
    (bind (_direction _newtrack_0) (`Timeline|leftCrushTimeline` :!via `PlayFromStart`)
      (:`Update`
        (`SceneComponent.K2_SetRelativeRotation` (`self.leftArmPivotPoint`) (`KismetMathLibrary.RLerp` (`self.leftArmStartingRotation`) (`self.leftArmHookRotation`) _newtrack_0) false false))
      (:`Finished`
        (bind (_direction_2 _timeline) (`Timeline|leftCrushTimeline2` :!via `PlayFromStart`)
          (:`Update`
            (`SceneComponent.K2_SetRelativeRotation` (`self.leftArmPivotPoint`) (`KismetMathLibrary.RLerp` (`self.leftArmHookRotation`) (`self.leftArmRaiseRotation`) _timeline) false false))
          (:`Finished`
            (`PrimitiveComponent.SetCollisionEnabled` _rightcrushcollision "NoCollision")
            (bind (_direction_3 _newtrack_0_2) (`Timeline|leftCrushReturn` :!via `PlayFromStart`)
              (:`Update`
                (`SceneComponent.K2_SetRelativeRotation` (`self.leftArmPivotPoint`) (`KismetMathLibrary.RLerp` (`self.leftArmHookRotation`) (`self.leftArmStartingRotation`) _newtrack_0_2) false false))
              (:`Finished`
                (set `self.leftHandInUse` false))))
          (:`NewTrack_1`
            (`GameplayStatics.PlayWorldCameraShake` "/Game/CoreSystems/BP_camerashake.BP_camerashake_C" (0.0 0.0 0.0) 0.0 (`self.Outer Radius`))
            (`GameplayStatics.PlaySoundAtLocation` "/Game/Sound/boss/CUE_smash.CUE_smash" (`SceneComponent.K2_GetComponentLocation` (`self.leftCrushCollision`)) (struct) 1.0 1.0 0.0 null null null))
          (:`enableCollision`
            (`PrimitiveComponent.SetCollisionEnabled` _rightcrushcollision "QueryOnly")))))))

(event `rightCrush`
  (if (not (`self.rightHandInUse`))
    (set `self.rightHandInUse` true)
    (bind (_direction _newtrack_0) (`Timeline|Timeline_3` :!via `PlayFromStart`)
      (:`Update`
        (`SceneComponent.K2_SetRelativeRotation` (`self.rightArmPivotPoint`) (`KismetMathLibrary.RLerp` (`self.rightArmStartingRotation`) (`self.rightArmHookRotation`) _newtrack_0) false false))
      (:`Finished`
        (bind (_direction_2 _timeline) (`Timeline|Timeline_0` :!via `PlayFromStart`)
          (:`Update`
            (`SceneComponent.K2_SetRelativeRotation` (`self.rightArmPivotPoint`) (`KismetMathLibrary.RLerp` (`self.rightArmHookRotation`) (`self.rightArmRaiseRotation`) _timeline) false false))
          (:`Finished`
            (`PrimitiveComponent.SetCollisionEnabled` (`self.leftCrushCollision`) "NoCollision")
            (bind (_direction_3 _newtrack_0_2) (`Timeline|Timeline_1` :!via `PlayFromStart`)
              (:`Update`
                (`SceneComponent.K2_SetRelativeRotation` (`self.rightArmPivotPoint`) (`KismetMathLibrary.RLerp` (`self.rightArmHookRotation`) (`self.rightArmStartingRotation`) _newtrack_0_2) false false))
              (:`Finished`
                (set `self.rightHandInUse` false))))
          (:`NewTrack_1`
            (`GameplayStatics.PlayWorldCameraShake` "/Game/CoreSystems/BP_camerashake.BP_camerashake_C" (0.0 0.0 0.0) 0.0 (`self.Outer Radius`))
            (`GameplayStatics.PlaySoundAtLocation` "/Game/Sound/boss/CUE_smash.CUE_smash" (`SceneComponent.K2_GetComponentLocation` (`self.rightCrushCollision`)) (struct) 1.0 1.0 0.0 null null null))
          (:`NewTrack_0`
            (`PrimitiveComponent.SetCollisionEnabled` (`self.rightCrushCollision`) "QueryOnly")))))))

(event `tryToRapidSmash`
  (`/Engine/EditorBlueprintResources/StandardMacros.DoOnce` false :!label _label_2
    (:`Completed`
      (bind _returnvalue (`KismetSystemLibrary.K2_SetTimerDelegate` (delegate `rapidSmash`) 0.1 true)))))

(event `resetSmash`
  (goto _label_2 :!via `Reset`))

(event `rapidSmash`
  (bind _crackeddecalmat (`self.crackedDecalMat`))
  (bind _crackeddecalmat2 (`self.crackedDecalMat2`))
  (if (and (not (`self.leftHandInUse`)) (not (`self.rightHandInUse`)))
    (`KismetSystemLibrary.K2_ClearAndInvalidateTimerHandle` (stale `tryToRapidSmash` _returnvalue))
    (set `self.leftHandInUse` true)
    (set `self.rightHandInUse` true)
    (bind (_direction _newtrack_0 _newtrack_2 _rightdecal _newtrack_3) (`Timeline|smash` :!via `PlayFromStart`)
      (:`Update`
        (`SceneComponent.K2_SetRelativeRotation` (`self.rightArmPivotPoint`) (`KismetMathLibrary.RLerp` (`self.rightArmStartingRotation`) (`self.rightArmRapidRotation`) _newtrack_0) false false)
        (`SceneComponent.K2_SetRelativeRotation` (`self.leftArmPivotPoint`) (`KismetMathLibrary.RLerp` (`self.leftArmStartingRotation`) (`self.leftArmRapidRotation`) _newtrack_2) false false)
        (`MaterialInstanceDynamic.SetScalarParameterValue` _crackeddecalmat "crackVisibility" _newtrack_3)
        (`MaterialInstanceDynamic.SetScalarParameterValue` _crackeddecalmat "crackAmount" _newtrack_3)
        (`MaterialInstanceDynamic.SetScalarParameterValue` _crackeddecalmat2 "crackVisibility" _rightdecal)
        (`MaterialInstanceDynamic.SetScalarParameterValue` _crackeddecalmat2 "crackAmount" _rightdecal))
      (:`Finished`
        (`PrimitiveComponent.SetCollisionEnabled` (`self.leftHookCollision`) "NoCollision")
        (`PrimitiveComponent.SetCollisionEnabled` (`self.rightHookCollision`) "NoCollision")
        (set `self.rightHandInUse` false)
        (set `self.leftHandInUse` false)
        (`KismetSystemLibrary.Delay` 0.5)
        (`self.resetSmash`))
      (:`screenshake`
        (`GameplayStatics.PlayWorldCameraShake` "/Game/CoreSystems/BP_camerashake.BP_camerashake_C" (0.0 0.0 0.0) 0.0 (`self.Outer Radius`))
        (`GameplayStatics.PlaySoundAtLocation` "/Game/Sound/boss/CUE_Crush.CUE_Crush" (`SceneComponent.K2_GetComponentLocation` (`self.weakPoint`)) (struct) 1.0 1.0 0.0 null null null))
      (:`collision`
        (`/Engine/EditorBlueprintResources/StandardMacros.FlipFlop`
          (:`A`
            (`PrimitiveComponent.SetCollisionEnabled` (`self.leftHookCollision`) "QueryOnly")
            (`PrimitiveComponent.SetCollisionEnabled` (`self.rightHookCollision`) "QueryOnly"))
          (:`B`
            (`PrimitiveComponent.SetCollisionEnabled` (`self.rightHookCollision`) "NoCollision")
            (`PrimitiveComponent.SetCollisionEnabled` (`self.leftHookCollision`) "NoCollision")))))))

(event `self.leftCrushCollision.OnComponentBeginOverlap`
  (params (OverlappedComponent :type "PrimitiveComponent Object Reference") (OtherActor :type "Actor Object Reference") (OtherComp :type "PrimitiveComponent Object Reference") (OtherBodyIndex :type Integer) (bFromSweep :type Boolean) (SweepResult :type "HitResult Structure (by ref)"))
  (bind _asbp_martyr (cast `/Game/SideScrollerBP/Blueprints/BP_Martyr` OtherActor))
  (if (== (`Character.CapsuleComponent` _asbp_martyr) OtherComp)
    (`/Game/SideScrollerBP/Blueprints/BP_Martyr.takeDamage` _asbp_martyr 50.0)))

(event `self.rightCrushCollision.OnComponentBeginOverlap`
  (params (OverlappedComponent :type "PrimitiveComponent Object Reference") (OtherActor :type "Actor Object Reference") (OtherComp :type "PrimitiveComponent Object Reference") (OtherBodyIndex :type Integer) (bFromSweep :type Boolean) (SweepResult :type "HitResult Structure (by ref)"))
  (bind _asbp_martyr (cast `/Game/SideScrollerBP/Blueprints/BP_Martyr` OtherActor))
  (if (== (`Character.CapsuleComponent` _asbp_martyr) OtherComp)
    (`/Game/SideScrollerBP/Blueprints/BP_Martyr.takeDamage` _asbp_martyr 50.0)))

(event `self.leftHookCollision.OnComponentBeginOverlap`
  (params (OverlappedComponent :type "PrimitiveComponent Object Reference") (OtherActor :type "Actor Object Reference") (OtherComp :type "PrimitiveComponent Object Reference") (OtherBodyIndex :type Integer) (bFromSweep :type Boolean) (SweepResult :type "HitResult Structure (by ref)"))
  (bind _asbp_martyr (cast `/Game/SideScrollerBP/Blueprints/BP_Martyr` OtherActor))
  (if (== (`Character.CapsuleComponent` _asbp_martyr) OtherComp)
    (`/Game/SideScrollerBP/Blueprints/BP_Martyr.takeDamage` _asbp_martyr 50.0)))

(event `self.rightHookCollision.OnComponentBeginOverlap`
  (params (OverlappedComponent :type "PrimitiveComponent Object Reference") (OtherActor :type "Actor Object Reference") (OtherComp :type "PrimitiveComponent Object Reference") (OtherBodyIndex :type Integer) (bFromSweep :type Boolean) (SweepResult :type "HitResult Structure (by ref)"))
  (bind _asbp_martyr (cast `/Game/SideScrollerBP/Blueprints/BP_Martyr` OtherActor))
  (if (== (`Character.CapsuleComponent` _asbp_martyr) OtherComp)
    (`/Game/SideScrollerBP/Blueprints/BP_Martyr.takeDamage` _asbp_martyr 50.0)))

(fn `UserConstructionScript`
  (bind (_leftarmstartingrotation_roll _leftarmstartingrotation_pitch _leftarmstartingrotation_yaw) (`KismetMathLibrary.BreakRotator` (`self.leftArmStartingRotation`)))
  (bind (_rightarmstartingrotation_roll _rightarmstartingrotation_pitch _rightarmstartingrotation_yaw) (`KismetMathLibrary.BreakRotator` (`self.rightArmStartingRotation`)))
  (bind _leftarmpivotpoint (`self.leftArmPivotPoint`))
  (bind _rightarmpivotpoint (`self.rightArmPivotPoint`))
  (bind _crackeddecalmat (`self.crackedDecalMat`))
  (`|ExecutionSequence`
    (:`then_0`
      (set `self.leftArmStartingLocation` (`SceneComponent.RelativeLocation` _leftarmpivotpoint))
      (bind _output_get (set `self.leftArmStartingRotation` (`SceneComponent.RelativeRotation` _leftarmpivotpoint)))
      (bind _output_get_2 (set `self.leftArmHookRotation` (`KismetMathLibrary.MakeRotator` (.roll _output_get) (.pitch _output_get) (+ (.yaw _output_get) -60.0))))
      (set `self.leftArmRaiseRotation` (`KismetMathLibrary.MakeRotator` (.roll _output_get_2) (+ (.pitch _output_get_2) -90.0) (.yaw _output_get_2)))
      (set `self.leftArmRapidRotation` (`KismetMathLibrary.MakeRotator` _leftarmstartingrotation_roll (+ _leftarmstartingrotation_pitch -40.0) _leftarmstartingrotation_yaw)))
    (:`then_1`
      (set `self.rightArmStartingLocation` (`SceneComponent.RelativeLocation` _rightarmpivotpoint))
      (bind _output_get_3 (set `self.rightArmStartingRotation` (`SceneComponent.RelativeRotation` _rightarmpivotpoint)))
      (bind _output_get_4 (set `self.rightArmHookRotation` (`KismetMathLibrary.MakeRotator` (.roll _output_get_3) (.pitch _output_get_3) (+ (.yaw _output_get_3) 60.0))))
      (set `self.rightArmRaiseRotation` (`KismetMathLibrary.MakeRotator` (.roll _output_get_4) (+ (.pitch _output_get_4) -90.0) (.yaw _output_get_4)))
      (set `self.rightArmRapidRotation` (`KismetMathLibrary.MakeRotator` _rightarmstartingrotation_roll (+ _rightarmstartingrotation_pitch -40.0) _rightarmstartingrotation_yaw)))
    (:`then_2`
      (bind _returnvalue (`KismetMaterialLibrary.CreateDynamicMaterialInstance` "/Game/Materials/MAT_crackedDecal_Inst.MAT_crackedDecal_Inst"))
      (set `self.crackedDecalMat` _returnvalue)
      (bind _returnvalue_2 (`KismetMaterialLibrary.CreateDynamicMaterialInstance` "/Game/Materials/MAT_crackedDecal_Inst.MAT_crackedDecal_Inst"))
      (set `self.crackedDecalMat2` _returnvalue_2)
      (`MaterialInstanceDynamic.SetScalarParameterValue` _crackeddecalmat "crackVisibility" 0.0)
      (`MaterialInstanceDynamic.SetScalarParameterValue` (`self.crackedDecalMat2`) "crackVisibility" 0.0)
      (`MaterialInstanceDynamic.SetScalarParameterValue` _crackeddecalmat "crackAmount" 0.0)
      (`MaterialInstanceDynamic.SetScalarParameterValue` (`self.crackedDecalMat2`) "crackAmount" 0.0))
    (:`then_3`
      (`PrimitiveComponent.SetCollisionEnabled` (`self.leftCrushCollision`) "NoCollision")
      (`PrimitiveComponent.SetCollisionEnabled` (`self.rightCrushCollision`) "NoCollision")
      (`PrimitiveComponent.SetCollisionEnabled` (`self.leftHookCollision`) "NoCollision")
      (`PrimitiveComponent.SetCollisionEnabled` (`self.rightHookCollision`) "NoCollision"))
    (:`then_4`
      (`TimelineComponent.SetPlayRate` (`self.moveBackwards`) 0.05))))