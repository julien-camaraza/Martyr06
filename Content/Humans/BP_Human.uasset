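; Rescuable human NPC that runs back and forth along a spline using two alternating timelines.
; It gathers enemies sharing its RoomNumber, and CheckEnemies scans their health to trigger the rescue, which runs it to the spline start and marks it Safe.
; A box overlap registers it as BP_Martyr's current Human while alive.
; Damage can kill it and update the HUD's lost count, while safe-room drop-off notifies the player and updates the checkpoint.
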(event `droppedOff`
  (if (`self.inASafeRoom`)
    (`/Engine/EditorBlueprintResources/StandardMacros.DoOnce` false
      (:`Completed`
        (`/Game/SideScrollerBP/Blueprints/BP_Martyr.humanPutInSafeRoom` (cast `/Game/SideScrollerBP/Blueprints/BP_Martyr` (`GameplayStatics.GetPlayerCharacter` 0) :!pure true))
        (`/Game/Humans/BP_safeRoom.updateCheckpont` (`self.safeRoom`))))))

(event `/Game/SideScrollerBP/Blueprints/BP_interface.takeDamage`
  (params (damage :type "Float (single-precision)"))
  (bind _returnvalue (- (`self.health`) damage))
  (set `self.health` _returnvalue)
  (if (<= _returnvalue 0.0)
    (`self.Die`)
    (`GameplayStatics.PlaySound2D` "/Game/Sound/SoundEffects/Human_Screams/Human_Dying_Cue.Human_Dying_Cue" 1.0 1.0 0.0 null null)
    (else
      (`KismetSystemLibrary.PrintString` (`KismetStringLibrary.Conv_DoubleToString` (`self.health`))))))

(event `self.Box.OnComponentEndOverlap`
  (params (OverlappedComponent :type "PrimitiveComponent Object Reference") (OtherActor :type "Actor Object Reference") (OtherComp :type "PrimitiveComponent Object Reference") (OtherBodyIndex :type Integer))
  (bind _asbp_martyr (cast `/Game/SideScrollerBP/Blueprints/BP_Martyr` (`GameplayStatics.GetPlayerCharacter` 0)))
  (if (== OtherComp (`Character.CapsuleComponent` _asbp_martyr))
    (set `/Game/SideScrollerBP/Blueprints/BP_Martyr.openStore` false _asbp_martyr)
    (`/Engine/EditorBlueprintResources/StandardMacros.IsValid` (`/Game/SideScrollerBP/Blueprints/BP_Martyr.human` _asbp_martyr)
      (:`Is Valid`
        (set `/Game/SideScrollerBP/Blueprints/BP_Martyr.human` null _asbp_martyr)
        (`KismetSystemLibrary.PrintString` (`KismetSystemLibrary.GetDisplayName` OtherComp))))))

(event `self.Box.OnComponentBeginOverlap`
  (params (OverlappedComponent :type "PrimitiveComponent Object Reference") (OtherActor :type "Actor Object Reference") (OtherComp :type "PrimitiveComponent Object Reference") (OtherBodyIndex :type Integer) (bFromSweep :type Boolean) (SweepResult :type "HitResult Structure (by ref)"))
  (bind _asbp_martyr (cast `/Game/SideScrollerBP/Blueprints/BP_Martyr` (`GameplayStatics.GetPlayerCharacter` 0) :!pure true))
  (if (`self.dead`)
    _
    (elif (== OtherComp (`Character.CapsuleComponent` _asbp_martyr))
      (`/Engine/EditorBlueprintResources/StandardMacros.IsValid` (`/Game/SideScrollerBP/Blueprints/BP_Martyr.human` _asbp_martyr)
        (:`Is Not Valid`
          (set `/Game/SideScrollerBP/Blueprints/BP_Martyr.human` self _asbp_martyr)
          (`KismetSystemLibrary.PrintString` (`KismetSystemLibrary.GetDisplayName` OtherComp)))))))

(event `self.ReceiveBeginPlay`
  (bind _runaround (`self.runAround`))
  (bind _runaround_2 (`self.runAround`))
  (`|ExecutionSequence`
    (:`then_0`
      (`TimelineComponent.SetPlayRate` (`self.movetimeline`) (`self.playRate`))
      (`TimelineComponent.SetPlayRate` (`self.Timeline_0`) (`self.playRate`))
      (`SkeletalMeshComponent.PlayAnimation` (`self.HumanMesh`) "/Game/Animations/Human/Human_Running.Human_Running" true)
      (bind (_direction _newtrack_0) (`Timeline|movetimeline` :!via `PlayFromStart` :!label _label)
        (:`Update`
          (set `self.distanceFromBase` _newtrack_0)
          (bind _returnvalue (`KismetMathLibrary.Lerp` 0.0 (`SplineComponent.GetSplineLength` (`self.runAround`)) _newtrack_0))
          (`SceneComponent.K2_SetWorldLocationAndRotation` (`self.HumanMesh`) (`SplineComponent.GetLocationAtDistanceAlongSpline` _runaround_2 _returnvalue "World") (`KismetMathLibrary.MakeRotator` (.roll (`SplineComponent.GetRotationAtDistanceAlongSpline` _runaround_2 _returnvalue "World")) (.pitch (`SplineComponent.GetRotationAtDistanceAlongSpline` _runaround_2 _returnvalue "World")) (+ (.yaw (`SplineComponent.GetRotationAtDistanceAlongSpline` _runaround_2 _returnvalue "World")) -90.0)) false false))
        (:`Finished`
          (bind (_direction_2 _newtrack_0_2) (`Timeline|Timeline_0` :!via `PlayFromStart` :!label _label_2)
            (:`Update`
              (set `self.distanceFromBase` _newtrack_0_2)
              (bind _returnvalue_2 (`KismetMathLibrary.Lerp` 0.0 (`SplineComponent.GetSplineLength` (`self.runAround`)) _newtrack_0_2))
              (`SceneComponent.K2_SetWorldLocationAndRotation` (`self.HumanMesh`) (`SplineComponent.GetLocationAtDistanceAlongSpline` _runaround _returnvalue_2 "World") (`KismetMathLibrary.MakeRotator` (.roll (`SplineComponent.GetRotationAtDistanceAlongSpline` _runaround _returnvalue_2 "World")) (.pitch (`SplineComponent.GetRotationAtDistanceAlongSpline` _runaround _returnvalue_2 "World")) (+ (.yaw (`SplineComponent.GetRotationAtDistanceAlongSpline` _runaround _returnvalue_2 "World")) 90.0)) false false))
            (:`Finished`
              (goto _label :!via `PlayFromStart`))))))
    (:`then_1`
      (bind _outactors (`GameplayStatics.GetAllActorsOfClass` "/Game/SideScrollerBP/Blueprints/BP_enemyParent2D.BP_enemyParent2D_C"))
      (for _array_element _outactors
        (if (== (`/Game/SideScrollerBP/Blueprints/BP_enemyParent2D.roomNumber` _array_element) (`self.roomNumber`))
          (`KismetArrayLibrary.Array_Add` (`self.scaryEnemies`) _array_element)))
      (`self.checkEnemies`))
    (:`then_2`
      (set `self.placeToSell` (`SplineComponent.GetLocationAtSplinePoint` (`self.goToSafeZone`) 1 "World")))))

(event `Die`
  (`/Game/NewMacros.DoOnce` false
    (:`Completed`
      (set `self.dead` true)
      (`|ExecutionSequence`
        (:`then_0`
          (goto _label :!via `Stop`))
        (:`then_1`
          (`SkeletalMeshComponent.PlayAnimation` (`self.HumanMesh`) "/Game/Geometry/Dying_Backwards.Dying_Backwards" false)
          (`ActorComponent.Activate` (`self.ParticleSystem`) false))
        (:`then_2`
          (goto _label_2 :!via `Stop`))
        (:`then_3`
          (bind _asbp_martyr (cast `/Game/SideScrollerBP/Blueprints/BP_Martyr` (`GameplayStatics.GetPlayerCharacter` 0)))
          (bind _result (`/Game/NewMacros.IncrementInt` (`/Game/SideScrollerBP/Blueprints/BP_Martyr.humansLost` _asbp_martyr))
            (:`  `
              (`/Game/UI/UI_HUD.updateHumanCount` (`/Game/SideScrollerBP/Blueprints/BP_Martyr.WIDHUD` _asbp_martyr) _result (`/Game/SideScrollerBP/Blueprints/BP_Martyr.humansSaved` _asbp_martyr) (`/Game/SideScrollerBP/Blueprints/BP_Martyr.humansToSave` _asbp_martyr)))))))))

(event `checkEnemies`
  (bind _array_element (`/Game/NewMacros.ForEachLoopWithBreakCom` (`self.scaryEnemies`) :!label _label_3)
    (:`LoopBody`
      (`/Engine/EditorBlueprintResources/StandardMacros.IsValid` _array_element
        (:`Is Valid`
          (if (<= (`/Game/SideScrollerBP/Blueprints/BP_enemyParent2D.enemyHealth` _array_element) 0.0)
            _
            (elif (`self.announceFear`)
              (`KismetSystemLibrary.PrintString` (`KismetSystemLibrary.GetDisplayName` _array_element))
              (goto _label_3 :!via `Break`)
              (else
                (goto _label_3 :!via `Break`)))))))
    (:`Completed`
      (if (not (`self.dead`))
        (`|ExecutionSequence`
          (:`then_0`
            (goto _label :!via `Stop`))
          (:`then_1`
            (goto _label_2 :!via `Stop`))
          (:`then_2`
            (`self.Saved`)
            (`GameplayStatics.PlaySoundAtLocation` "/Game/Sound/SoundEffects/Human_Thankyou/CUE_thankYou.CUE_thankYou" (`SceneComponent.K2_GetComponentLocation` (`self.HumanMesh`)) (struct) 1.0 1.0 0.0 null null null)))))))

(event `resetLocation`
  (bind _runaround (`self.runAround`))
  (`SceneComponent.K2_SetWorldLocationAndRotation` (`self.HumanMesh`) (`SplineComponent.GetLocationAtDistanceAlongSpline` _runaround 0.0 "World") (`KismetMathLibrary.MakeRotator` (.roll (`SplineComponent.GetRotationAtDistanceAlongSpline` _runaround 0.0 "World")) 0.0 (+ (.yaw (`SplineComponent.GetRotationAtDistanceAlongSpline` _runaround 0.0 "World")) 90.0)) false false))

(event `Saved`
  (bind _runaround (`self.runAround`))
  (bind (_direction _newtrack_0) (`Timeline|runBackToSafety` :!via `ReverseFromEnd`)
    (:`Update`
      (bind _returnvalue (`KismetMathLibrary.Lerp` 0.0 (`SplineComponent.GetSplineLength` (`self.runAround`)) (+ _newtrack_0 (`self.distanceFromBase`))))
      (`SceneComponent.K2_SetWorldLocationAndRotation` (`self.HumanMesh`) (`SplineComponent.GetLocationAtDistanceAlongSpline` _runaround _returnvalue "World") (`KismetMathLibrary.MakeRotator` (.roll (`SplineComponent.GetRotationAtDistanceAlongSpline` _runaround _returnvalue "World")) (.pitch (`SplineComponent.GetRotationAtDistanceAlongSpline` _runaround _returnvalue "World")) (+ (.yaw (`SplineComponent.GetRotationAtDistanceAlongSpline` _runaround _returnvalue "World")) 90.0)) false false))
    (:`Finished`
      (`self.resetLocation`)
      (set `self.safe` true)
      (`SkeletalMeshComponent.PlayAnimation` (`self.HumanMesh`) "/Game/Animations/Human/Human_Idle.Human_Idle" true))))

(fn `UserConstructionScript`)