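; Safe room volume that marks humans as sheltered and serves as a numbered checkpoint.
; On BeginPlay it registers itself in the GameInstance's checkpoint list.
; A Safe human entering the box gets InASafeRoom set and raises ActiveCheckpoint if this room's number is higher, printing the result.
; End overlap clears InASafeRoom only if OverlappedComponent, the box's own side of the overlap, equals the human's capsule.
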(event `self.ReceiveBeginPlay`
  (`KismetArrayLibrary.Array_AddUnique` (`/Game/SideScrollerBP/Blueprints/BP_GameInstance.checkpoints` (cast `/Game/SideScrollerBP/Blueprints/BP_GameInstance` (`GameplayStatics.GetGameInstance`) :!pure true)) self))

(event `self.Box.OnComponentBeginOverlap`
  (params (OverlappedComponent :type "PrimitiveComponent Object Reference") (OtherActor :type "Actor Object Reference") (OtherComp :type "PrimitiveComponent Object Reference") (OtherBodyIndex :type Integer) (bFromSweep :type Boolean) (SweepResult :type "HitResult Structure (by ref)"))
  (bind _asbp_game_instance (cast `/Game/SideScrollerBP/Blueprints/BP_GameInstance` (`GameplayStatics.GetGameInstance`) :!pure true))
  (bind _asbp_human (cast `/Game/Humans/BP_Human` OtherActor))
  (if (`/Game/Humans/BP_Human.safe` _asbp_human)
    (set `/Game/Humans/BP_Human.inASafeRoom` true _asbp_human)
    (if (< (`/Game/SideScrollerBP/Blueprints/BP_GameInstance.activeCheckpoint` _asbp_game_instance) (`self.checkpointNumber`))
      (bind _output_get (set `/Game/SideScrollerBP/Blueprints/BP_GameInstance.activeCheckpoint` (`self.checkpointNumber`) _asbp_game_instance))
      (`KismetSystemLibrary.PrintString` (`KismetTextLibrary.Conv_TextToString` (`|FormatText` "Active Checkpoint: {0}" _output_get))))))

(event `self.Box.OnComponentEndOverlap`
  (params (OverlappedComponent :type "PrimitiveComponent Object Reference") (OtherActor :type "Actor Object Reference") (OtherComp :type "PrimitiveComponent Object Reference") (OtherBodyIndex :type Integer))
  (bind _asbp_human (cast `/Game/Humans/BP_Human` OtherActor))
  (if (== OverlappedComponent (`Character.CapsuleComponent` _asbp_human))
    (set `/Game/Humans/BP_Human.inASafeRoom` false _asbp_human)))

(fn `UserConstructionScript`)